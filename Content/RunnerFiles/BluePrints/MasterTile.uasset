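; Endless-runner floor tile that fills three lanes on BeginPlay and extends the track as the player advances.
; SpawnObstacles chains random rolls per lane for pipes, boxes, coins or magnets; an empty roll skips remaining lanes, and most Lane 0 spawns have no class set.
; When the character overlaps Box, the game mode spawns another tile and adds multiplied points.
; The tile then raises walk speed within a clamp and destroys itself after a delay.
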(event OnComponentBeginOverlap(Box)
  (params (OverlappedComponent :type Primitive%20Component%20Object%20Reference) (OtherActor :type Actor%20Object%20Reference) (OtherComp :type Primitive%20Component%20Object%20Reference) (OtherBodyIndex :type Integer) (bFromSweep :type Boolean) (SweepResult :type Hit%20Result%20Structure%20%28by%20ref%29))
  ;[1 0.1771 0.3018] Spawn in new tile at location of new spawnpoint
  (Utilities|Casting|CastToThirdPersonCharacter OtherActor)
  (bind _asthird_person_game_mode (Utilities|Casting|CastToThirdPersonGameMode (Game|GetGameMode)))
  (Default|SpawnTile _asthird_person_game_mode)
  ;;[0.5521 0.3781 0.1692] Points Scoring System (When Pickup , multiply points. If not run across one tile = 1pt)
  (bind _asthird_person_game_mode_2 (Utilities|Casting|CastToThirdPersonGameMode (Game|GetGameMode)))
  (Variables|/Game/ThirdPersonBP/Blueprints/ThirdPersonGameMode.ThirdPersonGameMode_C|SetCurrentPoints _asthird_person_game_mode_2 (+ (* 10 (Variables|/Game/ThirdPersonBP/Blueprints/ThirdPersonGameMode.ThirdPersonGameMode_C|GetPointsMultiplier _asthird_person_game_mode_2)) (Variables|/Game/ThirdPersonBP/Blueprints/ThirdPersonGameMode.ThirdPersonGameMode_C|GetCurrentPoints _asthird_person_game_mode_2)))
  ;;[0.3907 0.2257 1] Increase walk speed after each tile
  (bind _asthird_person_character (Utilities|Casting|CastToThirdPersonCharacter (Game|GetPlayerCharacter 0)))
  (Variables|/Script/Engine.CharacterMovementComponent|SetMaxWalkSpeed (Variables|/Script/Engine.Character|GetCharacterMovement _asthird_person_character) (Math|Float|Clamp(Float) (* (Variables|/Script/Engine.CharacterMovementComponent|GetMaxWalkSpeed (Variables|/Script/Engine.Character|GetCharacterMovement _asthird_person_character)) 1.01) 6e+02 1.2e+03))
  (Utilities|FlowControl|Delay 0.5)
  (Actor|DestroyActor))

(event EventBeginPlay
  (CallFunction|SpawnObstacles))

(event Collision|EventActorBeginOverlap
  (params (OtherActor :type Actor%20Object%20Reference)))

(event EventTick
  (params (DeltaSeconds :type Float%20%28single-precision%29)))

(fn ConstructionScript)

(fn SpawnObstacles
  (bind _returnvalue (Math|Random|RandomFloatinRange 0.0 1.0))
  (bind _returnvalue_2 (Math|Random|RandomFloatinRange 0.0 1.0))
  (bind _returnvalue_3 (Math|Random|RandomFloatinRange 0.0 1.0))
  (bind _lane0 (Variables|Default|GetLane0))
  (bind _lane1 (Variables|Default|GetLane1))
  (bind _lane2 (Variables|Default|GetLane2))
  (bind _returnvalue_4 (Transformation|GetWorldTransform _lane0))
  (bind _returnvalue_5 (Transformation|GetWorldTransform _lane1))
  (bind _returnvalue_6 (Transformation|GetWorldTransform _lane2))
  ;[1 0.3345 0.89] Spawn Low Obstacles for Lane 0
  (if (Math|Float|InRange(Float) _returnvalue 0.0 0.4)
    (Game|SpawnActorfromClass "/Game/RunnerFiles/BluePrints/Obstacle_Pipe.Obstacle_Pipe_C" _returnvalue_4 "Undefined" 0 0)
    ;[1 0.3345 0.89] Spawn Low Obstacles for Lane 1
    (if (Math|Float|InRange(Float) _returnvalue_2 0.0 0.4) :!label _label
      (Game|SpawnActorfromClass "/Game/RunnerFiles/BluePrints/Obstacle_Pipe.Obstacle_Pipe_C" _returnvalue_5 "Undefined" 0 0)
      ;[1 0.3345 0.89] Spawn Low Obstacles for Lane 2
      (if (Math|Float|InRange(Float) _returnvalue_3 0.0 0.4) :!label _label_2
        (Game|SpawnActorfromClass "/Game/RunnerFiles/BluePrints/Obstacle_Pipe.Obstacle_Pipe_C" _returnvalue_6 "Undefined" 0 0)
        (elif (Math|Float|InRange(Float) _returnvalue_3 0.0 0.5)
          (Game|SpawnActorfromClass "/Game/RunnerFiles/BluePrints/Obstacle_Box.Obstacle_Box_C" _returnvalue_6 "Undefined" 0 0)
          (else
            ;[0.44 0.5941 1] Spawn Pickup
            (if (Math|Float|InRange(Float) _returnvalue_3 0.5 0.95)
              (Game|SpawnActorfromClass "/Game/RunnerFiles/BluePrints/Coin_Pickup.Coin_Pickup_C" _returnvalue_6 "Undefined" 0 0)
              (else
                ;[1 0.25 0.25] Spawn Magnet Pickup
                (if (Math|Float|InRange(Float) _returnvalue_3 0.95 1.0)
                  (Game|SpawnActorfromClass "/Game/RunnerFiles/BluePrints/Magnet_Pickup.Magnet_Pickup_C" _returnvalue_6 "Undefined" 0 0)))))))
      (elif (Math|Float|InRange(Float) _returnvalue_2 0.0 0.5)
        (Game|SpawnActorfromClass "/Game/RunnerFiles/BluePrints/Obstacle_Box.Obstacle_Box_C" _returnvalue_5 "Undefined" 0 0)
        (goto _label_2)
        (else
          ;[0.44 0.5941 1] Spawn Pickup
          (if (Math|Float|InRange(Float) _returnvalue_2 0.5 0.95)
            (Game|SpawnActorfromClass "/Game/RunnerFiles/BluePrints/Coin_Pickup.Coin_Pickup_C" _returnvalue_5 "Undefined" 0 0)
            (goto _label_2)
            (else
              ;[1 0.25 0.25] Spawn Magnet Pickup
              (if (Math|Float|InRange(Float) _returnvalue_2 0.95 1.0)
                (Game|SpawnActorfromClass "/Game/RunnerFiles/BluePrints/Magnet_Pickup.Magnet_Pickup_C" _returnvalue_5 "Undefined" 0 0)
                (goto _label_2)))))))
    (elif (Math|Float|InRange(Float) _returnvalue 0.0 0.5)
      (Game|SpawnActorfromClass "/Game/RunnerFiles/BluePrints/Obstacle_Box.Obstacle_Box_C" _returnvalue_4 "Undefined" 0 0)
      (goto _label)
      (else
        ;[0.44 0.5941 1] Spawn Pickup
        (if (Math|Float|InRange(Float) _returnvalue 0.5 0.95)
          (Game|SpawnActorfromClass "/Game/RunnerFiles/BluePrints/Coin_Pickup.Coin_Pickup_C" _returnvalue_4 "Undefined" 0 0)
          (goto _label)
          (else
            ;[1 0.25 0.25] Spawn Magnet Pickup
            (if (Math|Float|InRange(Float) _returnvalue 0.95 1.0)
              (Game|SpawnActorfromClass "/Game/RunnerFiles/BluePrints/Magnet_Pickup.Magnet_Pickup_C" _returnvalue_4 "Undefined" 0 0)
              (goto _label))))))))